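; BP_Light is a light prop whose static mesh colour is animated by a timeline after play begins.
; The construction script creates a dynamic instance of the Shine material and applies it to the mesh.
; On BeginPlay, it slows the Lighting timeline to one-fifth speed, waits for the Delay variable, then plays it.
; Each update writes the timeline's LightAlpha multiplied by Color into the material's Color parameter.
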(event `self.ReceiveBeginPlay`
  (`TimelineComponent.SetPlayRate` (`self.Lighting`) (/ 1.0 5.0))
  (`KismetSystemLibrary.Delay` (`self.Delay`))
  (bind (_direction _lightalpha) (`Timeline|Lighting`)
    (:`Update`
      (`MaterialInstanceDynamic.SetVectorParameterValue` (`self.DynamicMaterial`) "Color" (* _lightalpha (`self.Color`))))))

(fn `UserConstructionScript`
  (bind _returnvalue (`KismetMaterialLibrary.CreateDynamicMaterialInstance` "/Game/Extra_Assets/Frazier/Materials/Shine.Shine"))
  (bind _output_get (set `self.DynamicMaterial` _returnvalue))
  (`PrimitiveComponent.SetMaterial` (`self.StaticMesh`) 0 _output_get))